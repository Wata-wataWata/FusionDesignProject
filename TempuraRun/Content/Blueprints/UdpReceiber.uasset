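; UDP receiver actor that drives a RunCharacter with received speed, position and jump state.
; BeginPlay calls Connect, stores the result, caches the first RunCharacter found, then joins the Tick chain at the position write, skipping speed.
; While connected, Tick copies the three getter values onto that character.
; EndPlay calls Close.
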(event `self.ReceiveEndPlay`
  (params (EndPlayReason :type "EEndPlayReason Enum" :default "Destroyed"))
  (`self.Close`))

(event `self.ReceiveTick`
  (params (DeltaSeconds :type "Float (single-precision)"))
  (if (stale `self.ReceiveBeginPlay` _output_get)
    (bind _returnvalue (`self.GetSpeed`))
    (bind _returnvalue_2 (`self.GetPos`))
    (bind _returnvalue_3 (`self.GetIsJumping`))
    (set `/Game/ThirdPersonBP/Blueprints/RunCharacter.Speed` _returnvalue (stale `self.ReceiveBeginPlay` _asrun_character))
    (set `/Game/ThirdPersonBP/Blueprints/RunCharacter.Pos` _returnvalue_2 (stale `self.ReceiveBeginPlay` _asrun_character) :!label _label)
    (set `/Game/ThirdPersonBP/Blueprints/RunCharacter.IsJump` _returnvalue_3 (stale `self.ReceiveBeginPlay` _asrun_character))))

(event `self.ReceiveBeginPlay`
  (bind _returnvalue (`self.Connect`))
  (bind _output_get (set `self.isConected` _returnvalue))
  (bind _outactors (`GameplayStatics.GetAllActorsOfClass` "/Game/ThirdPersonBP/Blueprints/RunCharacter.RunCharacter_C"))
  (bind _asrun_character (cast `/Game/ThirdPersonBP/Blueprints/RunCharacter` (`|GetArrayItem` _outactors)))
  (goto _label))

(fn `UserConstructionScript`
  (locals (NewLocalVar_0 :type "Float (double-precision)" :default 0.0)))